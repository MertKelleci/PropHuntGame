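; Game mode for a Prop Hunt match that tracks joining players and randomly assigns one of them as the prop.
; PostLogin starts a short timer once at least two players are present and the game has not started.
; The chosen player's pawn is destroyed and replaced with a possessed BP_PropCharacter, then each player's HUD message is set by role.
; An invalid random pick retries selection after a delay.
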(event Custom|Start%20Game%20Timer
  ;[1 1 1] Game Logic
  ;;[1 1 1] Start game after 4 seconds
  (Utilities|Time|SetTimerbyEvent (delegate Custom|Select%20Prop%20Character) 4.0))

(event Custom|Select%20Prop%20Character
  (bind _playerlist (Variables|Default|GetPlayerList))
  ;[1 1 1] Game Logic
  ;;[1 1 1] Sellect a random player and assign them as prop
  (Variables|Default|SetGameStarted true)
  (bind _output_get (Variables|Default|SetProp%20Player (Utilities|Array|Get(acopy) _playerlist (Math|Random|RandomIntegerinRange 0 (Utilities|Array|Length _playerlist)))))
  (if (Utilities|IsValid _output_get)
    ;;[1 1 1] Spawn the player as prop at a location, destroy their original mesh and let them possess prop mesh
    (bind _returnvalue (Game|SpawnActorfromClass "/Game/Core/Blueprints/BP_PropCharacter.BP_PropCharacter_C" (Math|Transform|MakeTransform (Variables|Default|GetProp%20Spawn%20Location) "0, 0, 0" "1.000000,1.000000,1.000000") "Undefined" "MultiplyWithRoot" 0 0))
    (Actor|DestroyActor (Pawn|GetControlledPawn (Variables|Default|GetProp%20Player)))
    (Utilities|FlowControl|Delay 0.2)
    (Pawn|Possess (Variables|Default|GetProp%20Player) _returnvalue)
    ;;[1 1 1] Go through the player list and setup hud accordingly
    (Class|BPIPropHuntController|SetupPropWidget(Message) (Variables|Default|GetProp%20Player) true)
    (for _array_element (Variables|Default|GetPlayerList)
      (Utilities|IsValid _array_element
        (:Is%20Valid
          (bind _prop_player (Variables|Default|GetProp%20Player)
            (:then
              (if (!= _prop_player _array_element)
                (Class|BPIPropHuntController|SetupPropWidget(Message) _array_element false)))
            (:else)))))
    (else
      ;;[1 1 1] If prop actor is invalid, restart the game
      (Utilities|FlowControl|Delay 1.0)
      (CallFunction|SelectPropCharacter))))

(event EventPostLogin
  (params (NewPlayer :type Player%20Controller%20Object%20Reference))
  ;[1 1 1] Pre-Game Logic
  ;;[1 1 1] Add players to list
  (Utilities|Array|Add (Variables|Default|GetPlayerList) NewPlayer)
  ;;[1 1 1] If the game hasn't started yet and there are more than 2 players, start the game
  (if (not (Variables|Default|GetGameStarted))
    (if (>= (Utilities|Array|Length (Variables|Default|GetPlayerList)) 2)
      (CallFunction|StartGameTimer))))

(fn ConstructionScript)