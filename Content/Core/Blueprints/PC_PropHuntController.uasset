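; Player controller for a Prop Hunt game that owns the main HUD and relays match state to it.
; On BeginPlay it creates W_MainHUD for a local controller on authority or for any remote instance.
; Wrapper events pass prop role, health, countdown start and win result to OnClient events that update the HUD.
; It stores the IsProp role so the win screen knows the player's side.
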(event Custom|Set%20Prop%20On%20Client
  (params (Is%20Prop :type Boolean))
  (Default|SetupPropWidget (Variables|Default|GetMain%20Hud%20Ref) Is%20Prop))

(event Custom|Update%20Health%20On%20Client
  (params (Health :type Integer))
  (Default|UpdateHealthBar (Variables|Default|GetMain%20Hud%20Ref) Health))

(event Custom|Show%20Winscreen%20On%20Client
  (params (Prop%20Won :type Boolean) (Is%20Prop :type Boolean))
  (Default|ShowWinScreen (Variables|Default|GetMain%20Hud%20Ref) Prop%20Won Is%20Prop))

(event Custom|Start%20Countdown%20On%20Client
  (Default|StartTimer (Variables|Default|GetMain%20Hud%20Ref)))

(event EventBeginPlay
  (Networking|SwitchHasAuthority
    (:Authority
      (if (Pawn|IsLocalPlayerController)
        (bind _returnvalue (UserInterface|CreateWidget "/Game/Core/Widget/W_MainHUD.W_MainHUD_C" self :!label _label))
        (bind _output_get (Variables|Default|SetMain%20Hud%20Ref _returnvalue))
        (UserInterface|Viewport|AddtoViewport _output_get 0)))
    (:Remote
      (goto _label))))

(event EventShowWinScreenWidget
  (params (Prop%20Won :type Boolean))
  (CallFunction|ShowWinscreenonClient Prop%20Won (Variables|Default|GetIs%20Prop)))

(event EventSetupPropWidget
  (params (IsProp :type Boolean))
  (bind _output_get (Variables|Default|SetIs%20Prop IsProp))
  (CallFunction|SetProponClient _output_get))

(event EventUpdateHealthWidget
  (params (Health :type Integer))
  (CallFunction|UpdateHealthonClient Health))

(event EventStartCountdownWidget
  (CallFunction|StartCountdownonClient))

(fn ConstructionScript)